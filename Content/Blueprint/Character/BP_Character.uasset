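; Top-down player character Blueprint that handles movement-state input and a height-adjustable boom camera.
; Held walk, sprint and right-mouse aim inputs set flags and call ChangeMovementState, which is not defined in this graph.
; Mouse wheel zooms the boom between height limits through a looping timer that steps arm length, ignoring input mid-slide; instant CameraSlide is unused.
; The construction script configures the boom and lag, and F plays a camera shake.
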(event Input|ActionEvents|InputActionMovementModeChangeWalk
  (params (Key :type Key%20Structure :default "None"))
  (:Pressed
    (Variables|Default|SetWalkEnabled true)
    (Class|TDSProjectCharacter|ChangeMovementState :!label _label))
  (:Released
    (Variables|Default|SetWalkEnabled false)
    (goto _label)))

(event Input|ActionEvents|InputActionMovementModeChangeSprint
  (params (Key :type Key%20Structure :default "None"))
  (:Pressed
    (Variables|Default|SetSprintRunEnabled true)
    (Class|TDSProjectCharacter|ChangeMovementState :!label _label))
  (:Released
    (Variables|Default|SetSprintRunEnabled false)
    (goto _label)))

(event Input|AxisEvents|InputAxisMouseWheel
  (params (AxisValue :type Float%20%28single-precision%29))
  (CallFunction|CameraSlideSmooth AxisValue))

(event Input|KeyboardEvents|F
  (params (Key :type Key%20Structure :default "None"))
  (:Pressed
    (CallFunction|CameraShakeEvent)))

(event Input|MouseEvents|RightMouseButton
  (params (Key :type Key%20Structure :default "None"))
  (:Pressed
    (Variables|Default|SetAimEnabled true)
    (Class|TDSProjectCharacter|ChangeMovementState :!label _label))
  (:Released
    (Variables|Default|SetAimEnabled false)
    (goto _label)))

(fn ConstructionScript
  (bind _cameraboom (Variables|Default|GetCameraBoom))
  (bind _cameraboom_2 (Variables|Default|GetCameraBoom))
  (Variables|/Script/Engine.SpringArmComponent|SetTargetArmLength _cameraboom (Variables|Camera|Main|GetHeightCameraMin))
  (Transformation|SetRelativeRotation _cameraboom (Variables|Camera|Main|GetRotatorCamera) false false)
  (Variables|/Script/Engine.SpringArmComponent|SetbEnableCameraLag _cameraboom_2 (Variables|Camera|Main|GetFlow))
  (Variables|/Script/Engine.SpringArmComponent|SetCameraLagSpeed _cameraboom_2 (Variables|Camera|Main|GetCoefSmooth)))

(fn CameraShakeEvent
  (Camera|PlayWorldCameraShake "/Game/Blueprint/Game/BP_CameraShake.BP_CameraShake_C" (Transformation|GetWorldLocation (Variables|Default|GetTopDownCameraComponent)) 0.0 3e+01))

(fn CameraSlide
  (params (Value :type Float%20%28single-precision%29))
  (bind _heightcamerachangedistance (Variables|Camera|Slide|GetHeightCameraChangeDistance))
  (bind _cameraboom (Variables|Default|GetCameraBoom))
  (if (!= Value 0.0)
    (if (< Value 0.0)
      (if (>= (Variables|Camera|Main|GetHeightCameraMax) (+ (Variables|/Script/Engine.SpringArmComponent|GetTargetArmLength _cameraboom) _heightcamerachangedistance))
        (Variables|/Script/Engine.SpringArmComponent|SetTargetArmLength _cameraboom (+ (Variables|/Script/Engine.SpringArmComponent|GetTargetArmLength _cameraboom) _heightcamerachangedistance)))
      (elif (<= (Variables|Camera|Main|GetHeightCameraMin) (- (Variables|/Script/Engine.SpringArmComponent|GetTargetArmLength _cameraboom) _heightcamerachangedistance))
        (Variables|/Script/Engine.SpringArmComponent|SetTargetArmLength _cameraboom (- (Variables|/Script/Engine.SpringArmComponent|GetTargetArmLength _cameraboom) _heightcamerachangedistance))))))

(fn CameraSlideSmooth
  (params (Value :type Float%20%28single-precision%29))
  (bind _heightcamerachangedistance (Variables|Camera|Slide|GetHeightCameraChangeDistance))
  (bind _cameraboom (Variables|Default|GetCameraBoom))
  (bind _targetarmlength (Variables|/Script/Engine.SpringArmComponent|GetTargetArmLength _cameraboom))
  (if (Variables|Camera|Slide|GetSlideDone)
    (if (!= Value 0.0)
      (if (< Value 0.0)
        (if (>= (Variables|Camera|Main|GetHeightCameraMax) (+ _targetarmlength _heightcamerachangedistance))
          (Variables|Camera|Slide|SetSlideUp true)
          (Variables|Camera|Slide|SetSlideDone false :!label _label)
          (bind _returnvalue (Utilities|Time|SetTimerbyFunctionName 0 "CameraSlideSmoothTick" (Variables|Camera|Slide|GetTimerStep) true))
          (Variables|Camera|Slide|SetSlideTimer _returnvalue))
        (elif (<= (Variables|Camera|Main|GetHeightCameraMin) (- _targetarmlength _heightcamerachangedistance))
          (Variables|Camera|Slide|SetSlideUp false)
          (goto _label))))))

(fn CameraSlideSmoothTick
  (bind _hightcamerachangeslidestepdistance (Variables|Camera|Slide|GetHightCameraChangeSlideStepDistance))
  (bind _output_get (Variables|Camera|Slide|SetCurentSlideDistance (+ (Variables|Camera|Slide|GetCurentSlideDistance) _hightcamerachangeslidestepdistance)))
  (Variables|/Script/Engine.SpringArmComponent|SetTargetArmLength (Variables|Default|GetCameraBoom) (Math|Float|SelectFloat (+ (Variables|/Script/Engine.SpringArmComponent|GetTargetArmLength (Variables|Default|GetCameraBoom)) _hightcamerachangeslidestepdistance) (- (Variables|/Script/Engine.SpringArmComponent|GetTargetArmLength (Variables|Default|GetCameraBoom)) _hightcamerachangeslidestepdistance) (Variables|Camera|Slide|GetSlideUp)))
  (if (>= _output_get (Variables|Camera|Slide|GetHeightCameraChangeDistance))
    (Variables|Camera|Slide|SetCurentSlideDistance 0.0)
    (Variables|Camera|Slide|SetSlideDone true)
    (Utilities|Time|ClearandInvalidateTimerbyHandle (Variables|Camera|Slide|GetSlideTimer))))